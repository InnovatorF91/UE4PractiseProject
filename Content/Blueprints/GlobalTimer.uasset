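; GlobalTimer is a day-night clock for a survival game that turns game time into day, hour and minute, offset to start at 06:00.
; Each tick it rotates the sun light by time of day and updates the sky sphere, until StopTimer closes the gate.
; Crossing 06:00 or 18:00 flips IsDayTime and pushes a day or night message through SurvivalGameInstance.
; Sky light recapture and cubemap blending are disconnected, leaving UpdateSkyLight empty.
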(event `self.ReceiveBeginPlay`
  (bind _outactors (`GameplayStatics.GetAllActorsOfClass` "/Script/Engine.SkyLight"))
  (set `self.SkyLight` (`|GetArrayItem` _outactors)))

(event `self.ReceiveTick`
  (params (DeltaSeconds :type "Float (single-precision)"))
  (bind _secondsperday (`self.SecondsPerDay`))
  (bind _returnvalue (/ _secondsperday 24.0))
  (bind (_remainder _returnvalue_2) (`KismetMathLibrary.FMod` (+ (`KismetSystemLibrary.GetGameTimeInSeconds`) (/ _secondsperday 4.0)) _secondsperday))
  (bind (_remainder_2 _returnvalue_3) (`KismetMathLibrary.FMod` _remainder _returnvalue))
  (bind _returnvalue_4 (+ (* (/ _remainder _secondsperday) -360.0) 90.0))
  (`/Engine/EditorBlueprintResources/StandardMacros.Gate` false :!label _label
    (:`Exit`
      (`self.K2_SetActorRotation` (`self.SunLight`) (`KismetMathLibrary.MakeRotator` 0.0 _returnvalue_4) false)
      (`/Engine/EngineSky/BP_Sky_Sphere.UpdateSunDirection` (`self.SkySphere`))
      (`self.UpdateSkyLight` _returnvalue_4)
      (set `self.CurrentDay` _returnvalue_2)
      (bind _output_get (set `self.CurrentHour` _returnvalue_3))
      (set `self.CurrentMinute` (`.ReturnValue` (`KismetMathLibrary.FMod` _remainder_2 (/ _returnvalue 60.0))))
      (`|ExecutionSequence`
        (:`then_0`
          (if (`self.IsDayTime`)
            (bind _returnvalue_5 (and (>= _output_get 6) (< _output_get 18)))
            (if (not _returnvalue_5)
              (`self.EnterNightTime`))
            (elif _returnvalue_5
              (`self.EnterDayTime`))))
        (:`then_1`
          (set `self.IsDayTime` _returnvalue_5))))))

(event `StopTimer`
  (goto _label :!via `Close`))

(event `EnterDayTime`
  (`/Game/Blueprints/survivalGameInstance.PushMessage` (cast `/Game/Blueprints/survivalGameInstance` (`GameplayStatics.GetGameInstance`) :!pure true) "昼になった！"))

(event `EnterNightTime`
  (`/Game/Blueprints/survivalGameInstance.PushMessage` (cast `/Game/Blueprints/survivalGameInstance` (`GameplayStatics.GetGameInstance`) :!pure true) "夜になった！"))

(fn `UpdateSkyLight`
  (params (LightDirection :type "Float (double-precision)")))

(fn `UserConstructionScript`)