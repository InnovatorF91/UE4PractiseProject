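; Survival game instance that owns and toggles the game's UI panels: runtime HUD, message box, pickable, inventory, cabinet and failure screens.
; Named events route through shared ShowPanel and HidePanel functions, which lazily create each widget into a by-ref variable and reuse it.
; An active-panel counter switches to Game-and-UI input with a cursor for interactive panels, restoring game-only input when HidePanel brings it to zero.
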(event `ShowRunTimeUI`
  (`self.ShowPanel` "/Game/UI/UI_RunTimeUI.UI_RunTimeUI_C" (`self.RunTimeUI`))
  (`self.ShowPanel` "/Game/UI/UI_MessageBox.UI_MessageBox_C" (`self.MessageBox`)))

(event `PushMessage`
  (params (textContent :type String))
  (`/Game/UI/UI_MessageBox.PushMessage` (`self.MessageBox`) textContent))

(event `ShowPickablePanel`
  (`self.ShowPanel` "/Game/UI/UI_PickablePanel.UI_PickablePanel_C" (`self.PickablePanel`) true))

(event `HidePickablePanel`
  (`self.HidePanel` (`self.PickablePanel`)))

(event `ShowInventoryPanel`
  (`self.ShowPanel` "/Game/UI/UI_Inventory.UI_Inventory_C" (`self.InventoryPanel`) true))

(event `HideInventoryPanel`
  (`self.HidePanel` (`self.InventoryPanel`)))

(event `ShowCabinetPannel`
  (`self.ShowPanel` "/Game/UI/UI_Cabinet.UI_Cabinet_C" (`self.CabinetUI`) true))

(event `HideCabinetPannel`
  (`self.HidePanel` (`self.CabinetUI`)))

(event `ShowFailedPannel`
  (`self.ShowPanel` "/Game/UI/UI_Failed.UI_Failed_C" (`self.FailedPannel`) true))

(event `HideAllPannel`
  (`self.HidePanel` (`self.PickablePanel`))
  (`self.HidePanel` (`self.InventoryPanel`))
  (`self.HidePanel` (`self.CabinetUI`)))

(fn `HidePanel`
  (params (PanelVar :type "Widget Object Reference"))
  (bind _returnvalue (`GameplayStatics.GetPlayerController` 0))
  (`/Engine/EditorBlueprintResources/StandardMacros.IsValid` PanelVar
    (:`Is Valid`
      (if (`Widget.IsVisible` PanelVar)
        (`Widget.RemoveFromParent` PanelVar)
        (bind _result (`/Engine/EditorBlueprintResources/StandardMacros.DecrementInt` (`self.ActiveUICount`))
          (:`  `
            (if (== _result 0)
              (`WidgetBlueprintLibrary.SetInputMode_GameOnly` _returnvalue)
              (set `PlayerController.bShowMouseCursor` false _returnvalue))))))))

(fn `ShowPanel`
  (params (PannelTypeClass :type "UserWidget Class Reference") (PanelVariable :type "UserWidget Object Reference (by ref)") (bChangeUIMode :type Boolean))
  (bind _returnvalue (`GameplayStatics.GetPlayerController` 0))
  (`/Engine/EditorBlueprintResources/StandardMacros.IsValid` PanelVariable
    (:`Is Valid`
      (if (not (`Widget.IsInViewport` PanelVariable))
        (`UserWidget.AddToViewport` PanelVariable 0 :!label _label)
        (if bChangeUIMode
          (`/Engine/EditorBlueprintResources/StandardMacros.IncrementInt` (`self.ActiveUICount`)
            (:`  `
              (`WidgetBlueprintLibrary.SetInputMode_GameAndUIEx` _returnvalue PanelVariable)
              (set `PlayerController.bShowMouseCursor` true _returnvalue))))))
    (:`Is Not Valid`
      (bind _returnvalue_2 (`|CreateWidget` PannelTypeClass (`GameplayStatics.GetPlayerController` 0)))
      (`|VariableSetRef` PanelVariable _returnvalue_2)
      (goto _label))))