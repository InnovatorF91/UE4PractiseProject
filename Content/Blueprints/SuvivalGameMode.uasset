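; Game mode for a survival game that handles game over, restarting MainLevel and quitting.
; BeginPlay shows the runtime UI through SurvivalGameInstance and caches the level's GlobalTimer and Cabinet actors.
; GameOver stops the timer and shows the failed panel with survived day, hour and a Japanese record message.
; CheckScore compares total hours against the bestScore save slot, saving new or first records and returning that message.
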(event `self.ReceiveBeginPlay`
  (`|ExecutionSequence`
    (:`then_0`
      (bind _outactors (`GameplayStatics.GetAllActorsOfClass` "/Game/Blueprints/GlobalTimer.GlobalTimer_C"))
      (set `self.GlobelTimer` (`|GetArrayItem` _outactors))
      (`/Game/Blueprints/survivalGameInstance.ShowRunTimeUI` (cast `/Game/Blueprints/survivalGameInstance` (`GameplayStatics.GetGameInstance`) :!pure true)))
    (:`then_1`
      (bind _outactors_2 (`GameplayStatics.GetAllActorsOfClass` "/Game/Blueprints/Props/Cabinet.Cabinet_C"))
      (set `self.Cabinet` (`|GetArrayItem` _outactors_2)))
    (:`then_2`
      (set `self.As Survival Game Instance` (cast `/Game/Blueprints/survivalGameInstance` (`GameplayStatics.GetGameInstance`) :!pure true)))))

(event `GameOver`
  (bind _as_survival_game_instance (`self.As Survival Game Instance`))
  (bind _globeltimer (`self.GlobelTimer`))
  (bind _currentday (`/Game/Blueprints/GlobalTimer.CurrentDay` _globeltimer))
  (bind _currenthour (`/Game/Blueprints/GlobalTimer.CurrentHour` _globeltimer))
  (`/Game/Blueprints/GlobalTimer.StopTimer` (`self.GlobelTimer`))
  (`/Game/Blueprints/survivalGameInstance.HideAllPannel` _as_survival_game_instance)
  (`/Game/Blueprints/survivalGameInstance.ShowFailedPannel` _as_survival_game_instance)
  (bind _recordtext (`self.CheckScore` _currentday _currenthour))
  (`/Game/UI/UI_Failed.SetTexts` (`/Game/Blueprints/survivalGameInstance.FailedPannel` _as_survival_game_instance) _currentday _currenthour _recordtext))

(event `RestartGame`
  (`GameplayStatics.OpenLevel` "MainLevel"))

(event `QuitGame`
  (`KismetSystemLibrary.ExecuteConsoleCommand` "exit" null))

(fn `CheckScore`
  (params (newDay :type Integer) (newHour :type Integer))
  (returns (RecordText :type String))
  (bind _returnvalue (`GameplayStatics.DoesSaveGameExist` "bestScore"))
  (if _returnvalue
    (bind _returnvalue_2 (`GameplayStatics.LoadGameFromSlot` "bestScore"))
    (bind _asbest_score (cast `/Game/Blueprints/BestScore` _returnvalue_2))
    (bind _bestday (`/Game/Blueprints/BestScore.BestDay` _asbest_score))
    (bind _besthour (`/Game/Blueprints/BestScore.BestHour` _asbest_score))
    (bind _returnvalue_3 (- (+ (* newDay 24) newHour) (+ (* _bestday 24) _besthour)))
    (if (> _returnvalue_3 0)
      _
      (elif (== _returnvalue_3 0)
        (return "もう少し頑張ってください！")
        (else
          (return (`KismetStringLibrary.Concat_StrStr` "一番長いサバイバル時間：" (`KismetStringLibrary.Conv_IntToString` _bestday) "日" (`KismetStringLibrary.Conv_IntToString` _besthour) "時"))))))
  (bind _returnvalue_4 (`GameplayStatics.CreateSaveGameObject` "/Game/Blueprints/BestScore.BestScore_C"))
  (set `/Game/Blueprints/BestScore.BestDay` newDay _returnvalue_4)
  (set `/Game/Blueprints/BestScore.BestHour` newHour _returnvalue_4)
  (`GameplayStatics.SaveGameToSlot` _returnvalue_4 "bestScore")
  (return "おめでとうございます！新記録を作りました！"))

(fn `UserConstructionScript`)